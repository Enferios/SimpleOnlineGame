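; BP_DoorSlider is a sliding door that opens along its local Y axis and closes itself after a delay.
; Init caches the mesh's closed position at BeginPlay and derives the open position from OpeningOffset.
; OpenDoor plays a timeline that lerps between the two, with each update feeding a delay that calls CloseDoor to reverse it.
; Interact only forwards to the parent implementation.
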(event `self.ReceiveBeginPlay`
  (`self.Init`))

(event `self.OpenDoor`
  ;[1 1 1] Opening / closing
  (bind (_direction _alpha) (`Timeline|DoorTimeline` :!label _label)
    (:`Update`
      (`SceneComponent.K2_SetRelativeLocation` (`self.DoorMesh`) (`KismetMathLibrary.VLerp` (`self.DoorMeshClosedPosition`) (`self.DoorMeshOpenedPosition`) _alpha) false false)
      (`KismetSystemLibrary.Delay` (`self.DelayBeforeClose`))
      (`self.CloseDoor`))))

(event `self.CloseDoor`
  ;[1 1 1] Opening / closing
  (goto _label :!via `Reverse`))

(event `InteractableInterface.Interact`
  (params (Interactor :type "Actor Object Reference"))
  ;[1 1 1] Opening / closing
  (`parent.Interact` Interactor))

(fn `Init`
  (bind _output_get (set `self.DoorMeshClosedPosition` (`SceneComponent.RelativeLocation` (`self.DoorMesh`))))
  (set `self.DoorMeshOpenedPosition` (`KismetMathLibrary.MakeVector` (.x _output_get) (+ (`self.OpeningOffset`) (.y _output_get)) (.z _output_get))))

(fn `UserConstructionScript`)